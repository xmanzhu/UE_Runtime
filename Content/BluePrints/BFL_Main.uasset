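; Blueprint function library with a helper that returns the world location under the mouse cursor.
; It scales the viewport mouse position by the viewport scale and deprojects it through player controller 0 into a world ray.
; A long Visibility line trace along that ray returns the hit location, and only the hit case sets a return value.
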(fn LineTraceReturnLocation
  (bind _returnvalue (Class|WidgetLayoutLibrary|GetMousePositiononViewport))
  (bind (_outhit _returnvalue_2) (Collision|LineTraceByChannel 0 (.WorldPosition (Class|GameplayStatics|DeprojectScreentoWorld (Game|GetPlayerController 0) (* _returnvalue (Class|WidgetLayoutLibrary|GetViewportScale)))) (+ (.WorldPosition (Class|GameplayStatics|DeprojectScreentoWorld (Game|GetPlayerController 0) (* _returnvalue (Class|WidgetLayoutLibrary|GetViewportScale)))) (* (.WorldDirection (Class|GameplayStatics|DeprojectScreentoWorld (Game|GetPlayerController 0) (* _returnvalue (Class|WidgetLayoutLibrary|GetViewportScale)))) 1e+04)) "TraceTypeQuery1" false 0 "None"))
  (if _returnvalue_2
    (return (.Location (Collision|BreakHitResult _outhit)))))