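; BP_BaseMovement lets the player drag a chosen actor with the left mouse button, currently along the X axis.
; Pressing takes TargetActor from BP_CollectInfoFromMouse and opens a Tick gate that moves it while IsChosen holds; releasing closes the gate.
; CastToWorld intersects the deprojected mouse ray with an axis-aligned plane through the actor, supporting plane or single-axis constraints, though Tick always passes X.
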(event EventBeginPlay
  (bind _returnvalue (Game|GetPlayerController 0))
  (bind _outactors (Actor|GetAllActorsOfClass "/Game/BluePrints/BP_CollectInfoFromMouse.BP_CollectInfoFromMouse_C"))
  (bind _output_get (Variables|Default|SettempMouseVector _outactors))
  (Variables|Default|SetMouseInfo (Utilities|Array|Get(acopy) _output_get))
  (Input|SetInputModeGameOnly _returnvalue false)
  (Class|GameplayStatics|SetViewportMouseCaptureMode "CaptureDuringMouseDown")
  (Input|EnableInput _returnvalue))

(event Collision|EventActorBeginOverlap
  (params (OtherActor :type Actor%20Object%20Reference)))

(event EventTick
  (params (DeltaSeconds :type Float%20%28single-precision%29))
  (bind _target_actor (Variables|Default|GetTarget%20Actor))
  (if (Variables|/Game/BluePrints/BP_CollectInfoFromMouse.BP_CollectInfoFromMouse_C|GetIsChosen (Variables|Default|GetMouseInfo))
    (Utilities|FlowControl|Gate true
      (:Exit
        (if (Utilities|IsValid _target_actor)
          (bind _resultlocation (CallFunction|CasttoWorld "x" (Transformation|GetActorLocation _target_actor)))
          (Transformation|SetActorLocation (Variables|Default|GetTarget%20Actor) _resultlocation false false))))))

(event Input|MouseEvents|LeftMouseButton
  (params (Key :type Key%20Structure :default "None"))
  (:Pressed
    (Default|MButtonPress (Variables|Default|GetMouseInfo))
    (Variables|Default|SetTarget%20Actor (Variables|/Game/BluePrints/BP_CollectInfoFromMouse.BP_CollectInfoFromMouse_C|GetTargetActor (Variables|Default|GetMouseInfo)))
    (Utilities|FlowControl|Gate true) ; enters at Open
  )
  (:Released
    (Utilities|FlowControl|Gate true) ; enters at Close
  ))

(fn ConstructionScript)

(fn CasttoWorld
  (params (MoveType :type String) (Actor :type Vector))
  (bind _returnvalue (Game|GetPlayerController 0))
  (bind (_worldlocation _worlddirection) (Game|Player|ConvertMouseLocationToWorldSpace _returnvalue))
  (LocalVariables|SetMove MoveType)
  (LocalVariables|SetActorL Actor)
  (LocalVariables|SetWorldLoc _worldlocation)
  (LocalVariables|SetWorldDirec _worlddirection)
  (switch string (LocalVariables|GetMove)
    (:xoy
      ;[1 1 1] 由摄像机位置与角度计算鼠标位置映射到空间内
      (LocalVariables|SettempLocation (.Z (Math|Vector|BreakVector (LocalVariables|GetWorldLoc))) :!label _label)
      (LocalVariables|SettempDirection (.Z (Math|Vector|BreakVector (LocalVariables|GetWorldDirec))))
      (LocalVariables|SetActorLoc (.Z (Math|Vector|BreakVector (LocalVariables|GetActorL)))))
    (:xoz
      (LocalVariables|SettempLocation (.Y (Math|Vector|BreakVector (LocalVariables|GetWorldLoc))))
      (LocalVariables|SetActorLoc (.Y (Math|Vector|BreakVector (LocalVariables|GetActorL))))
      (LocalVariables|SettempDirection (.Y (Math|Vector|BreakVector (LocalVariables|GetWorldDirec)))))
    (:yoz
      (LocalVariables|SettempLocation (.X (Math|Vector|BreakVector (LocalVariables|GetWorldLoc))) :!label _label_2)
      (LocalVariables|SettempDirection (.X (Math|Vector|BreakVector (LocalVariables|GetWorldDirec))))
      (LocalVariables|SetActorLoc (.X (Math|Vector|BreakVector (LocalVariables|GetActorL)))))
    (:x
      (goto _label))
    (:y
      (goto _label))
    (:z
      (goto _label_2)))
  (LocalVariables|SetPreResult (+ (* (/ (* (- (LocalVariables|GettempLocation) (LocalVariables|GetActorLoc)) (LocalVariables|GetWorldDirec)) (LocalVariables|GettempDirection)) -1.0) (LocalVariables|GetWorldLoc)))
  (switch string (LocalVariables|GetMove)
    (:xoy
      _)
    (:xoz
      _)
    (:yoz
      _)
    (:x
      (LocalVariables|SetPreResult (Math|Vector|MakeVector (.x (LocalVariables|GetPreResult)) (.y (LocalVariables|GetActorL)) (.z (LocalVariables|GetPreResult)))))
    (:y
      (LocalVariables|SetPreResult (Math|Vector|MakeVector (.x (LocalVariables|GetActorL)) (.y (LocalVariables|GetPreResult)) (.z (LocalVariables|GetPreResult)))))
    (:z
      (LocalVariables|SetPreResult (Math|Vector|MakeVector (.x (LocalVariables|GetPreResult)) (.y (LocalVariables|GetActorL)) (.z (LocalVariables|GetPreResult))))))
  (return (LocalVariables|GetPreResult)))