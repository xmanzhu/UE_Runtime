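; BP_Music is a music player actor that plays tracks through a media player and shows the current media name on a text render.
; MusicBegin opens a fixed first track and sets IsOpen, which gates track switching.
; MusicLeft steps forward and MusicRight backward through the wrapping Musics array, MusicByIndex selects directly, and separate events play or pause.
; Tick compares the media name with the displayed text and refreshes it on change.
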(event Custom|ShowMusicName
  ;[1 1 1] 函数：展示媒体名
  (bind _output_get (Variables|Default|SetMusicText (Utilities|Text|ToText(String) (Utilities|String|Append "Playing:" (Utilities|String|ToString(Text) (Class|MediaPlayer|GetMediaName (Variables|Default|GetMusicPlayer)))))))
  (Rendering|Components|TextRender|SetText (Variables|Default|GetTextRender1) _output_get))

(event Custom|MusicPause
  ;[1 1 1] 函数：音乐继续播放和暂停
  (Sequencer|Player|Pause (Variables|Default|GetMusicPlayer)))

(event Custom|MusicContinue
  ;[1 1 1] 函数：音乐继续播放和暂停
  (Media|MediaPlayer|Play (Variables|Default|GetMusicPlayer) :!class /Script/MediaAssets.MediaPlayer))

(event Custom|MusicLeft
  ;[1 1 1] 函数：切换音乐
  (if (Variables|Default|GetIsOpen)
    (bind _output_get (Variables|Default|Setmusicindex (Math|Integer|%(Integer) (+ (Variables|Default|Getmusicindex) 1) (Utilities|Array|Length (Variables|Default|Getmusics)))))
    (Media|MediaPlayer|OpenSource (Variables|Default|GetMusicPlayer) (Utilities|Array|Get(acopy) (Variables|Default|Getmusics) _output_get))))

(event Custom|MusicBegin
  ;[1 1 1] 函数：打开音乐播放器
  (Media|MediaPlayer|OpenSource (Variables|Default|GetMusicPlayer) "/Game/Assets/Music/Love_Story-Taylor_Swift.Love_Story-Taylor_Swift")
  (Variables|Default|SetIsPlaying true)
  (Variables|Default|Setmusicindex 0)
  (Variables|Default|SetIsOpen true))

(event Custom|MusicRight
  (bind _musics (Variables|Default|Getmusics))
  (bind _returnvalue (Utilities|Array|Length _musics))
  ;[1 1 1] 函数：切换音乐
  (if (Variables|Default|GetIsOpen)
    (bind _output_get (Variables|Default|Setmusicindex (Math|Integer|%(Integer) (+ (Variables|Default|Getmusicindex) (- _returnvalue 1)) _returnvalue)))
    (Media|MediaPlayer|OpenSource (Variables|Default|GetMusicPlayer) (Utilities|Array|Get(acopy) (Variables|Default|Getmusics) _output_get))))

(event EventBeginPlay
  ;[1 1 1] 开始时将音乐播放器绑定到变量上
  (Variables|Default|SetMusicPlayer "/Game/Assets/Music/MusicPlayer.MusicPlayer")
  (CallFunction|ShowMusicName))

(event Collision|EventActorBeginOverlap
  (params (OtherActor :type Actor%20Object%20Reference)))

(event EventTick
  (params (DeltaSeconds :type Float%20%28single-precision%29))
  ;[1 1 1] tick时刻判断媒体名是否发生变化
  (if (not (Utilities|Enum|Equal(Enum) (Utilities|String|ToString(Text) (Utilities|Text|ToText(String) (Utilities|String|Append "Playing:" (Utilities|String|ToString(Text) (Class|MediaPlayer|GetMediaName (Variables|Default|GetMusicPlayer)))))) (Utilities|String|ToString(Text) (Variables|Default|GetMusicText))))
    (CallFunction|ShowMusicName)))

(fn ConstructionScript)

(fn MusicbyIndex
  (params (index :type Integer))
  ;[1 1 1] 函数：通过索引值来播放制定音乐
  (if (Variables|Default|GetIsOpen)
    (bind _output_get (Variables|Default|Setmusicindex index))
    (Media|MediaPlayer|OpenSource (Variables|Default|GetMusicPlayer) (Utilities|Array|Get(acopy) (Variables|Default|Getmusics) _output_get))))