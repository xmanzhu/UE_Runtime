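; BP_BaseRotation is a base Blueprint for click-triggered rotation, with an empty DoRotation event as the rotation step.
; Activation binds to clicks on OwnerActor, falling back to OwnerComp if the actor is invalid.
; Component clicks call TryRotation for any button, while the actor click handler is empty and a left-button check follows its binding in activation.
; TryRotation starts a looping DoRotation timer only when none exists.
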(event Custom|activation
  (bind _owneractor (Variables|Default|GetOwnerActor)
    (:then
      (EventDispatchers|AssignOnClicked _owneractor (delegate Custom|OnClicked_actor))
      (if (== (stale Custom|OnClicked_actor ButtonPressed) "LeftMouseButton")
        (CallFunction|TryRotation)))
    (:else
      (bind _ownercomp (Variables|Default|GetOwnerComp)
        (:then
          (EventDispatchers|AssignOnClicked _ownercomp (delegate Custom|OnClicked_Comp)))
        (:else)))))

(event Custom|OnClicked_actor
  (params (TouchedActor :type Actor%20Object%20Reference) (ButtonPressed :type Key%20Structure :default "None")))

(event Custom|OnClicked_Comp
  (params (TouchedComponent :type Primitive%20Component%20Object%20Reference) (ButtonPressed :type Key%20Structure :default "None"))
  (if true
    (CallFunction|TryRotation)))

(event Custom|TryRotation
  (if (not (Utilities|Time|IsValidTimerHandle (Variables|Default|GetTimerRotation)))
    (bind _returnvalue (Utilities|Time|SetTimerbyEvent (delegate Custom|DoRotation) (Variables|Default|GetTime) true))
    (Variables|Default|SetTimerRotation _returnvalue)))

(event Custom|DoRotation)

(fn ConstructionScript)