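; BP_CollectInfoFromMouse is an actor that records which actor sits under the mouse cursor when clicked.
; On BeginPlay it shows the cursor, enables click events, sets game-only input with mouse capture during mouse down, and enables its own input.
; The M_Button press event runs a complex Visibility trace under the cursor and stores the hit actor in TargetActor.
; Release and Tick are empty, and nothing here uses the stored target.
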(event Custom|M_ButtonPress
  (Variables|Default|SetTargetActor (.HitActor (Collision|BreakHitResult (.HitResult (Game|Player|GetHitResultUnderCursorbyChannel (Variables|Default|GetPlayerController) "TraceTypeQuery1" true))))))

(event Custom|M_ButtonRelease)

(event EventBeginPlay
  (bind _returnvalue (Game|GetPlayerController 0))
  (Variables|Default|SetPlayerController _returnvalue)
  (Variables|/Script/Engine.PlayerController|SetbShowMouseCursor (Variables|Default|GetPlayerController) true)
  (Variables|/Script/Engine.PlayerController|SetbEnableClickEvents (Variables|Default|GetPlayerController) true)
  (Input|SetInputModeGameOnly _returnvalue false)
  (Class|GameplayStatics|SetViewportMouseCaptureMode "CaptureDuringMouseDown")
  (Input|EnableInput (Variables|Default|GetPlayerController)))

(event Collision|EventActorBeginOverlap
  (params (OtherActor :type Actor%20Object%20Reference)))

(event EventTick
  (params (DeltaSeconds :type Float%20%28single-precision%29)))

(fn ConstructionScript)