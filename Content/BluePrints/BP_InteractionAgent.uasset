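; BP_InteractionAgent turns a left mouse press into a move or rotation interaction on the actor under mouse selection.
; On BeginPlay it caches the first BP_CollectInfoFromMouse, enables input and sets game-only mode with capture during mouse down.
; Each press updates that mouse helper, reads its TargetActor, then constructs and activates a MoveAbility or RotationAbility object, chosen by the Rotation variable and given the PC_Rotation controller.
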(event EventBeginPlay
  (bind _returnvalue (Game|GetPlayerController 0))
  (bind _outactors (Actor|GetAllActorsOfClass "/Game/BluePrints/BP_CollectInfoFromMouse.BP_CollectInfoFromMouse_C"))
  (bind _output_get (Variables|Default|SetTemp%20Mouse%20Vector _outactors))
  (Variables|Default|SetMouse%20Info (Utilities|Array|Get(acopy) _output_get))
  (Input|SetInputModeGameOnly _returnvalue false)
  (Class|GameplayStatics|SetViewportMouseCaptureMode "CaptureDuringMouseDown")
  (Input|EnableInput _returnvalue))

(event Input|MouseEvents|LeftMouseButton
  (params (Key :type Key%20Structure :default "None"))
  (bind _mouse_info (Variables|Default|GetMouse%20Info))
  (:Pressed
    (Default|MButtonPress _mouse_info)
    (bind _aspc_rotation (Utilities|Casting|CastToPC_Rotation (Game|GetPlayerController 0)))
    (Variables|Default|SetAs%20PC%20Rotation _aspc_rotation)
    (Variables|Default|SetTarget%20Actor (Variables|/Game/BluePrints/BP_CollectInfoFromMouse.BP_CollectInfoFromMouse_C|GetTargetActor _mouse_info))
    (switch Utilities|FlowControl|Switch|SwitchonInteractiveMode "NewEnumerator1"
      (:NewEnumerator0
        (bind _returnvalue (Game|ConstructObjectfromClass "/Game/BluePrints/Ability/MoveAbility.MoveAbility_C" "NewEnumerator0" (Variables|Default|GetAs%20PC%20Rotation) (Variables|Default|GetTarget%20Actor)))
        (bind _output_get (Variables|Default|SetAgentObject _returnvalue))
        (bind _asmove_ability (Utilities|Casting|CastToMoveAbility _output_get))
        (Default|Activation _asmove_ability))
      (:NewEnumerator1
        (bind _returnvalue_2 (Game|ConstructObjectfromClass "/Game/BluePrints/Ability/RotationAbility.RotationAbility_C" (Variables|Default|GetTarget%20Actor) "NewEnumerator0" (Variables|Default|GetAs%20PC%20Rotation)))
        (bind _output_get_2 (Variables|Default|SetAgentObject _returnvalue_2))
        (bind _asrotation_ability (Utilities|Casting|CastToRotationAbility _output_get_2))
        (Default|Activation _asrotation_ability)))))

(fn ConstructionScript)