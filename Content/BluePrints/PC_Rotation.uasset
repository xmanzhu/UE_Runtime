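; PC_Rotation is a player controller that exposes mouse input to other objects, apparently for a rotation interaction.
; On left mouse button release it calls OnLeftMouseButtonRelease, which looks like an event dispatcher for listeners.
; Helper functions return input axis values as mouse X and Y, and the cursor's deprojected world location and direction.
; The controller applies no rotation itself, and its BeginPlay and Tick events are empty.
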(event EventBeginPlay)

(event EventTick
  (params (DeltaSeconds :type Float%20%28single-precision%29)))

(event Input|MouseEvents|LeftMouseButton
  (params (Key :type Key%20Structure :default "None"))
  (:Released
    (Default|CallOnLeftMouseButtonRelease)))

(fn ConstructionScript)

(fn GetMouseX
  (return (Class|Actor|GetInputAxisKeyValue)))

(fn GetMouseY
  (return (Class|Actor|GetInputAxisKeyValue)))

(fn GetMouseInfo
  (bind _self self)
  (bind (_worldlocation _worlddirection) (Game|Player|ConvertMouseLocationToWorldSpace _self))
  (return _worldlocation _worlddirection))